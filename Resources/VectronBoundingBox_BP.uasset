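; VectronBoundingBox_BP is a bounding box actor that debug-draws a voxel vector field.
; On BeginPlay it loops over the Vectors in its referenced content, converting each flat index to grid coordinates and then to a voxel position.
; Non-zero vectors appear as fixed-length arrows showing direction only, and zero vectors as points.
; The drawing happens once with a long duration, with no per-tick update.
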(event EventBeginPlay
  (for (_array_element _array_index) (.vectors (Variables|Default|Getm_contentReference))
    (bind _returnvalue (Class|VectronBoundingBox|GetResolvedIndex _array_index))
    (bind _returnvalue_2 (Class|VectronBoundingBox|GetVoxelPosition (Math|Float|Floor (.x _returnvalue)) (Math|Float|Floor (.y _returnvalue)) (Math|Float|Floor (.z _returnvalue))))
    (Variables|Default|SetVoxelPosition _returnvalue_2)
    (if (Math|Vector|NotEqual(Vector) (* (Math|Vector|Normalize _array_element) 2e+01) "0, 0, 0" 0.0001)
      (Rendering|Debug|DrawDebugArrow (Variables|Default|GetVoxelPosition) (+ (* (Math|Vector|Normalize _array_element) 2e+01) (Variables|Default|GetVoxelPosition)) 2.0 "(R=0.000000,G=0.000000,B=0.000000,A=1.000000)" 1e+02)
      (else
        (Rendering|Debug|DrawDebugPoint :Position (Variables|Default|GetVoxelPosition) :Size 5.0 :Duration 1e+02)))))

(event EventActorBeginOverlap
  (params (OtherActor :type Actor%20Object%20Reference)))

(event EventTick
  (params (DeltaSeconds :type Float%20%28single-precision%29)))

(fn ConstructionScript)